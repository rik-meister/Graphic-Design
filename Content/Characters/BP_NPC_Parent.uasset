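; BP_NPC_Parent is a base NPC that reacts when the player comes within talking range.
; Entering the dialogue sphere adds a glow overlay, shows a widget, disables movement, sets a blackboard range flag and plays a timeline turning the NPC toward the player.
; Any end overlap or non-player entry hides the widget and glow, then after a delay applies one rotation step and restores walking, leaving the flag set.
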(event `self.ReceiveBeginPlay`
  ;[1 1 1] Establishes Player and hides widget on start
  (set `self.Player` (`GameplayStatics.GetPlayerCharacter` 0))
  ;;[1 1 1] Added for testing, delete later
  (`KismetSystemLibrary.Delay` 0.2)
  (`SceneComponent.SetHiddenInGame` (`self.Widget`) true false))

(event `self.DialogueSphereCollision.OnComponentBeginOverlap`
  (params (OverlappedComponent :type "PrimitiveComponent Object Reference") (OtherActor :type "Actor Object Reference") (OtherComp :type "PrimitiveComponent Object Reference") (OtherBodyIndex :type Integer) (bFromSweep :type Boolean) (SweepResult :type "HitResult Structure (by ref)"))
  (bind _returnvalue (`self.K2_GetActorLocation`))
  (bind _widget (`self.Widget`))
  (bind _charactermovement (`self.CharacterMovement`))
  ;[1 1 1] Checks for Player that is established, should only pop up when player is near
  (if (== (`GameplayStatics.GetObjectClass` OtherActor) "/Game/ThirdPerson/Blueprints/BP_ThirdPersonCharacter.BP_ThirdPersonCharacter_C")
    (`MeshComponent.SetOverlayMaterial` (`self.Mesh`) "/Game/Materials/M_Glow.M_Glow")
    (`BlackboardComponent.SetValueAsBool` (`AIBlueprintHelperLibrary.GetBlackboard` null) "EnterInteractRange" true)
    (`CharacterMovementComponent.DisableMovement` _charactermovement)
    (`SceneComponent.SetHiddenInGame` _widget false false)
    (`Timeline|RotateToPlayer`
      (:`Update`
        (`self.K2_SetActorRotation` (`KismetMathLibrary.RInterpTo` (`self.K2_GetActorRotation`) (`KismetMathLibrary.FindLookAtRotation` (`self.K2_GetActorLocation`) (`self.K2_GetActorLocation` (`GameplayStatics.GetPlayerCharacter` 0))) (`GameplayStatics.GetWorldDeltaSeconds`) 5.0))))
    (else
      (`SceneComponent.SetHiddenInGame` _widget true false :!label _label)
      (`MeshComponent.SetOverlayMaterial` (`self.Mesh`) null)
      (`KismetSystemLibrary.Delay` 2.0)
      (`self.K2_SetActorRotation` (`KismetMathLibrary.RInterpTo` (`self.K2_GetActorRotation`) (`KismetMathLibrary.FindLookAtRotation` _returnvalue (`KismetMathLibrary.GetForwardVector` (`KismetMathLibrary.Conv_VectorToRotator` _returnvalue))) (`GameplayStatics.GetWorldDeltaSeconds`) 10.0))
      (`CharacterMovementComponent.SetMovementMode` _charactermovement "MOVE_Walking" 0))))

(event `self.DialogueSphereCollision.OnComponentEndOverlap`
  (params (OverlappedComponent :type "PrimitiveComponent Object Reference") (OtherActor :type "Actor Object Reference") (OtherComp :type "PrimitiveComponent Object Reference") (OtherBodyIndex :type Integer))
  ;[1 1 1] Checks for Player that is established, should only pop up when player is near
  (goto _label))

(fn `UserConstructionScript`)