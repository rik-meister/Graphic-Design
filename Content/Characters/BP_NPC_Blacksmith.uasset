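; Blacksmith NPC Blueprint that shows its dialogue lines on screen through a Talk event.
; Each Talk increments DialogueIndex, creates and caches a WBP_Dialogue widget if none is valid, and writes the current Dialogue entry into its text block.
; The index increments again after display, so successive calls skip entries.
; When the incremented index reaches the end of the array, Talk removes the widget from the viewport.
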(event `/Game/Interfaces/BPI_Dialogue.Talk`
  (`/Engine/EditorBlueprintResources/StandardMacros.IncrementInt` (`self.DialogueIndex`)
    (:`  `
      (if (< (`self.DialogueIndex`) (`KismetArrayLibrary.Array_Length` (`self.Dialogue`)))
        (`self.UI` :!label _label
          (:`then`
            _)
          (:`else`
            (bind _returnvalue (`|CreateWidget` "/Game/Widgets/WBP_Dialogue.WBP_Dialogue_C" (`GameplayStatics.GetPlayerController` 0)))
            (bind _output_get (set `self.UI` _returnvalue))
            (`UserWidget.AddToViewport` _output_get 0)))
        (`TextBlock.SetText` (`/Game/Widgets/WBP_Dialogue.Dialogue_TextBlock` (`self.UI`)) (`KismetTextLibrary.Conv_StringToText` (`|GetArrayItem` (`self.Dialogue`) (`self.DialogueIndex`))))
        (`/Engine/EditorBlueprintResources/StandardMacros.IncrementInt` (`self.DialogueIndex`)
          (:`  `
            (if (> (`self.DialogueIndex`) (`KismetArrayLibrary.Array_Length` (`self.Dialogue`)))
              (set `self.DialogueIndex` (`self.DialogueIndex`))
              (goto _label))))
        (else
          (`Widget.RemoveFromParent` (`self.UI`)))))))

(fn `UserConstructionScript`
  (`parent.UserConstructionScript`))